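; Player character for the space shooter, handling movement, firing and damage from enemy bullets.
; Enhanced Input drives movement along the actor's forward and right vectors, and DoFire spawns ammo at the Firepoint, with a timer enforcing the fire delay.
; Overlaps with actors tagged "Balaenemigo" broadcast Onplayerdestroy and remove a life.
; When lives reach zero, it notifies BP_GameMode through PlayerDead.
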(event `self.ReceiveBeginPlay`
  (bind _asbp_player_controller (cast `/Game/00_Space_shooter/BP_PlayerController` (`self.GetController`)))
  (bind _returnvalue (pcsubsystem `EnhancedInputLocalPlayerSubsystem` _asbp_player_controller))
  (`/Engine/EditorBlueprintResources/StandardMacros.IsValid` _returnvalue
    (:`Is Valid`
      (`EnhancedInputSubsystemInterface.AddMappingContext` _returnvalue "/Game/00_Space_shooter/input/BP_input_mapping.BP_input_mapping" 0 (struct)))))

(event `self.ReceiveActorBeginOverlap`
  (params (OtherActor :type "Actor Object Reference"))
  (if (`KismetArrayLibrary.Array_Contains` (`Actor.Tags` OtherActor) "Balaenemigo")
    (`self.onplayerdestroy`)
    (cast `/Game/00_Space_shooter/BP_GameMode` (`GameplayStatics.GetGameMode`))
    (`self.DamageActor`)))

(event `EnhancedInput|/Game/00_Space_shooter/input/BP_InputMove`
  (params (ActionValue :type "Vector2D Structure") (ElapsedSeconds :type "Float (double-precision)") (TriggeredSeconds :type "Float (double-precision)") (InputAction :type "InputAction Object Reference" :default "/Game/00_Space_shooter/input/BP_InputMove.BP_InputMove"))
  (:`Triggered`
    (`self.AddMovementInput` (`self.GetActorRightVector`) ActionValue_X)
    (`self.AddMovementInput` (`self.GetActorForwardVector`) ActionValue_Y)))

(event `EnhancedInput|/Game/00_Space_shooter/input/BP_InputFire`
  (params (ActionValue :type Boolean) (ElapsedSeconds :type "Float (double-precision)") (TriggeredSeconds :type "Float (double-precision)") (InputAction :type "InputAction Object Reference" :default "/Game/00_Space_shooter/input/BP_InputFire.BP_InputFire"))
  (:`Triggered`
    (if (`self.canfire`)
      (`self.DoFire`)
      (set `self.canfire` false)
      (`KismetSystemLibrary.K2_SetTimerDelegate` (delegate `Updatefire`) (`self.firedelay`)))))

(event `Updatefire`
  (set `self.canfire` true))

(event `DamageActor`
  (bind _output_get (set `self.Lifes` (- (`self.Lifes`) 1)))
  (if (== _output_get 0)
    (bind _asbp_game_mode (cast `/Game/00_Space_shooter/BP_GameMode` (`GameplayStatics.GetGameMode`)))
    (`/Game/00_Space_shooter/BP_GameMode.PlayerDead` _asbp_game_mode)))

(fn `DoFire`
  (`|SpawnActorFromClass` (`self.ammo`) (`SceneComponent.K2_GetComponentToWorld` (`self.firepoint`)) "Undefined" "MultiplyWithRoot" null null))

(fn `UserConstructionScript`)