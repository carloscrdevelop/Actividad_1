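; Player pawn for a space shooter, driven by Enhanced Input.
; On BeginPlay it casts the controller to BP_PlayerController and adds the input mapping context.
; The move action stores its 2D value and clears it on release, and Tick offsets the location along right and forward vectors by Speed and delta time, without sweep.
; The fire action only prints a debug string.
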(event `self.ReceiveBeginPlay`
  (bind _asbp_player_controller (cast `/Game/00_Space_shooter/BP_PlayerController` (`self.GetController`)))
  (bind _returnvalue (pcsubsystem `EnhancedInputLocalPlayerSubsystem` _asbp_player_controller))
  (`/Engine/EditorBlueprintResources/StandardMacros.IsValid` _returnvalue
    (:`Is Valid`
      (`EnhancedInputSubsystemInterface.AddMappingContext` _returnvalue "/Game/00_Space_shooter/input/BP_input_mapping.BP_input_mapping" 0 (struct)))))

(event `self.ReceiveTick`
  (params (DeltaSeconds :type "Float (single-precision)"))
  (bind (_inputsaved_x _inputsaved_y) (`KismetMathLibrary.BreakVector2D` (`self.inputSaved`)))
  (bind _returnvalue (* DeltaSeconds (`self.Speed`)))
  (`self.K2_SetActorLocation` (+ (+ (* (`self.GetActorRightVector`) (* _returnvalue _inputsaved_x)) (* (* _returnvalue _inputsaved_y) (`self.GetActorForwardVector`))) (`self.K2_GetActorLocation`))))

(event `EnhancedInput|/Game/00_Space_shooter/input/BP_InputFire`
  (params (ActionValue :type Boolean) (ElapsedSeconds :type "Float (double-precision)") (TriggeredSeconds :type "Float (double-precision)") (InputAction :type "InputAction Object Reference" :default "/Game/00_Space_shooter/input/BP_InputFire.BP_InputFire"))
  (:`Triggered`
    (`KismetSystemLibrary.PrintString` "disparo")))

(event `EnhancedInput|/Game/00_Space_shooter/input/BP_InputMove`
  (params (ActionValue :type "Vector2D Structure") (ElapsedSeconds :type "Float (double-precision)") (TriggeredSeconds :type "Float (double-precision)") (InputAction :type "InputAction Object Reference" :default "/Game/00_Space_shooter/input/BP_InputMove.BP_InputMove"))
  (:`Triggered`
    (set `self.inputSaved` ActionValue))
  (:`Canceled`
    (set `self.inputSaved` (0.0 0.0) :!label _label))
  (:`Completed`
    (goto _label)))

(fn `UserConstructionScript`)