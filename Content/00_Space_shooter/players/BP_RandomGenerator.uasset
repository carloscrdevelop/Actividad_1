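; BP_RandomGenerator is an enemy spawner actor for the space shooter.
; A looping timer started on BeginPlay calls SpawnEnemy, which spawns at a random component tagged "Spawnpoint".
; The enemy class comes from a random index bounded by the game mode's Level and clamped to MaxNumEnemies.
; An event that shortens the spawn interval exists, but its binding to enemy destruction is unconnected, and the running timer is never reset.
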(event `self.ReceiveBeginPlay`
  (`KismetSystemLibrary.K2_SetTimerDelegate` (delegate `Spawn`) (`self.SpawNTime`) true)
  (cast `/Game/00_Space_shooter/BP_GameMode` (`GameplayStatics.GetGameMode`)))

(event `Spawn`
  (`self.SpawnEnemy`))

(event `EnemyDestroeyed`
  (set `self.SpawNTime` (- (`self.SpawNTime`) 1.0)))

(fn `GetClassToSpawn`
  (params (Type :type Integer))
  (returns (ReturnValue :type "/Game/00_Space_shooter/players/BP_Enemybase Class Reference"))
  (return (select `int` (`KismetMathLibrary.Clamp` Type 0 (`self.MaxNumEnemies`)) :`0` "/Game/00_Space_shooter/players/BP_Enemybase.BP_Enemybase_C" :`1` "/Game/00_Space_shooter/players/BP_EnemyH.BP_EnemyH_C" :`2` null :!type "/Game/00_Space_shooter/players/BP_Enemybase Class Reference")))

(fn `SpawnEnemy`
  (returns (EnemySpawned :type "/Game/00_Space_shooter/players/BP_Enemybase Object Reference"))
  (bind _returnvalue (`self.GetComponentsByTag` "/Script/Engine.SceneComponent" "Spawnpoint"))
  (bind _returnvalue_2 (`self.GetClassToSpawn` (`KismetMathLibrary.RandomInteger` (`/Game/00_Space_shooter/BP_GameMode.level` (`self.m_GameMode`)))))
  (bind _returnvalue_3 (`|SpawnActorFromClass` _returnvalue_2 (`SceneComponent.K2_GetComponentToWorld` (`|GetArrayItem` _returnvalue (`KismetMathLibrary.RandomInteger` (`KismetArrayLibrary.Array_Length` _returnvalue)))) "Undefined" "MultiplyWithRoot" null null))
  (bind _asbp_enemybase (cast `/Game/00_Space_shooter/players/BP_Enemybase` _returnvalue_3))
  (return _asbp_enemybase))

(fn `UserConstructionScript`)