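; BP_Enemybase is a space shooter enemy that flies straight along its initial forward vector and fires periodically.
; Tick moves it without sweeping and runs a timer that spawns Ammo at Firepoint, matching the enemy's rotation.
; Overlapping a Player-tagged actor calls the OnEnemyDestroy dispatcher, whose bound event destroys it after a short delay, and notifies BP_GameMode.
; An ammo-cast check for the same destroy path is left disconnected.
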(event `self.ReceiveBeginPlay`
  (set `self.MovementVector` (`self.GetActorForwardVector`))
  (add `self.OnEnemyDestroy` (delegate `Destroyed_event`)))

(event `Destroyed_event`
  (`KismetSystemLibrary.Delay` 0.1)
  (`self.K2_DestroyActor`))

(event `self.ReceiveActorBeginOverlap`
  (params (OtherActor :type "Actor Object Reference"))
  (if (`KismetArrayLibrary.Array_Contains` (`Actor.Tags` OtherActor) "Player")
    (`self.OnEnemyDestroy`)
    (bind _asbp_game_mode (cast `/Game/00_Space_shooter/BP_GameMode` (`GameplayStatics.GetGameMode`)))
    (`/Game/00_Space_shooter/BP_GameMode.EnemyDestroyed` _asbp_game_mode)))

(event `self.ReceiveTick`
  (params (DeltaSeconds :type "Float (single-precision)"))
  (`self.move` DeltaSeconds)
  (bind _output_get (set `self.shootcurrenttime` (+ DeltaSeconds (`self.shootcurrenttime`))))
  (if (> _output_get (`self.delayshoot`))
    (set `self.shootcurrenttime` 0.0)
    (`self.fire`)))

(fn `fire`
  (bind _returnvalue (`|SpawnActorFromClass` (`self.ammo`) (`SceneComponent.K2_GetComponentToWorld` (`self.firepoint`)) "Undefined" "MultiplyWithRoot" null null))
  (`self.K2_SetActorRotation` _returnvalue (`self.K2_GetActorRotation`) false))

(fn `move`
  (params (DeltaTime :type "Float (double-precision)"))
  (`self.K2_SetActorLocation` (+ (`self.K2_GetActorLocation`) (* (* DeltaTime (`self.speed`)) (`self.MovementVector`)))))

(fn `UserConstructionScript`)