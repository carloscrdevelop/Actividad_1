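; Game mode for a space shooter that tracks progress, enemy kills and level, and relays player death to the HUD.
; Tick steadily adds a per-tick increment to Progress.
; EnemyDestroyed counts kills and raises Level on every second one.
; PlayerDead casts the first player controller's HUD to BP_SpaceS_HUB and calls PlayerKilled on it.
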(event `self.ReceiveTick`
  (params (DeltaSeconds :type "Float (single-precision)"))
  (set `self.Progress` (+ (`self.Progress`) (`self.IncrementPerTick`))))

(event `PlayerDead`
  (bind _asbp_space_s_hub (cast `/Game/00_Space_shooter/UI/BP_SpaceS_HUB` (`PlayerController.GetHUD` (`GameplayStatics.GetPlayerController` 0))))
  (`/Game/00_Space_shooter/UI/BP_SpaceS_HUB.PlayerKilled` _asbp_space_s_hub))

(event `EnemyDestroyed`
  (bind _output_get (set `self.EnemiesDestroyed` (+ (`self.EnemiesDestroyed`) 1)))
  (if (== (mod _output_get 2) 0)
    (set `self.level` (+ (`self.level`) 1))))

(fn `UserConstructionScript`)